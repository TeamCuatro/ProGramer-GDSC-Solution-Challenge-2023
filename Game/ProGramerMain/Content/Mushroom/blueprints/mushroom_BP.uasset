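; Ranged mushroom enemy character that turns to face the player each tick until dead and fires projectiles.
; Player entry into its box starts a looping timer that plays the attack animation unless dead or falling; a separate event spawns the projectile at the spawn point.
; Damage updates a widget health bar shown briefly, applies knockback and jumps animation states.
; Death hides the bar, changes collision and destroys the actor after a delay.
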(event OnComponentBeginOverlap(Box)
  (params (OverlappedComponent :type Primitive%20Component%20Object%20Reference) (OtherActor :type Actor%20Object%20Reference) (OtherComp :type Primitive%20Component%20Object%20Reference) (OtherBodyIndex :type Integer) (bFromSweep :type Boolean) (SweepResult :type Hit%20Result%20Structure%20%28by%20ref%29))
  ;[1 1 1] Attack
  (if (== OtherActor (Game|GetPlayerCharacter 0))
    (Utilities|Time|SetTimerbyEvent (delegate Custom|mushroomattack) 1.5 true)))

(event Custom|handleroation
  ;[1 1 1] Handle rotation
  (if (not (Variables|Donotedit|Getisdead))
    (if (< (.x (Math|Vector|GetUnitDirection(Vector) (Transformation|GetActorLocation (Game|GetPlayerCharacter 0)) (Transformation|GetActorLocation))) 0.0)
      (Transformation|SetActorRotation "0, 0, 0")
      (else
        (Transformation|SetActorRotation "0,180.000000, 0")))))

(event Custom|mushroomattack
  ;[1 1 1] Attack
  (if (not (or (Variables|Donotedit|Getisdead) (AI|Components|NavMovement|IsFalling (Variables|Character|GetCharacterMovement))))
    (Class|PaperZDAnimInstance|JumptoNode (Variables|/Script/PaperZD.PaperZDAnimationComponent|GetAnimInstance (Variables|Default|GetAnimationComponent)) (Variables|Edit|Getrangedattack) "None")))

(event Custom|Spawnprojectile
  ;[1 1 1] Attack
  (Game|SpawnActorfromClass (Variables|Edit|GetProjectiles) (Math|Transform|MakeTransform (Transformation|GetWorldLocation (Variables|Default|Getspawnpoint)) (Transformation|GetActorRotation) "1.000000,1.000000,1.000000") "Undefined" 0 0))

(event EventTick
  (params (DeltaSeconds :type Float%20%28single-precision%29))
  ;[1 1 1] Event tick
  (CallFunction|Handleroation))

(event EventBeginPlay
  ;[1 1 1] Event begin play set up
  (Variables|Edit|Setmaxhealth (Variables|edit|Gethealth))
  (bind _asrangedenemyhealthbar_wb (Utilities|Casting|CastToRangedenemyhealthbar_WB (UserInterface|GetWidget (Variables|Default|GetWidget))))
  (bind _output_get (Variables|donotedit|SetAs%20Rangedenemyhealthbar%20WB _asrangedenemyhealthbar_wb))
  (Variables|/Game/Widgetblueprints/Rangedenemyhealthbar_WB.Rangedenemyhealthbar_WB_C|SetMushrromref _output_get self))

(event Game|Damage|EventAnyDamage
  (params (Damage :type Float%20%28single-precision%29) (DamageType :type Damage%20Type%20Object%20Reference) (InstigatedBy :type Controller%20Object%20Reference) (DamageCauser :type Actor%20Object%20Reference))
  ;[1 1 1] Handle damage
  (Variables|edit|Sethealth (- (Variables|edit|Gethealth) Damage))
  (Default|Updatehealthbar (Variables|donotedit|GetAs%20Rangedenemyhealthbar%20WB))
  (Variables|Donotedit|Setenemydamaged true)
  (if (<= (Variables|edit|Gethealth) 0.0)
    (Class|PaperZDAnimInstance|JumptoNode (Variables|/Script/PaperZD.PaperZDAnimationComponent|GetAnimInstance (Variables|Default|GetAnimationComponent)) (Variables|Edit|Getdeath) "None")
    (Variables|Donotedit|Setisdead true)
    (Rendering|SetVisibility (Variables|Default|GetWidget) false false)
    (Collision|SetCollisionProfileName (Variables|Default|GetCapsuleComponent) "OverlapOnlyPawn" true :!class /Script/Engine.PrimitiveComponent)
    (Utilities|FlowControl|Delay 3.0)
    (Actor|DestroyActor)
    (else
      (Character|LaunchCharacter (Math|Vector|MakeVector (* (select (< (.x (Math|Vector|GetUnitDirection(Vector) (Transformation|GetActorLocation DamageCauser) (Transformation|GetActorLocation))) 0.0) 1.0 -1.0) -1.2e+03) 0.0 3e+02) true true)
      (Class|PaperZDAnimInstance|JumptoNode (Variables|/Script/PaperZD.PaperZDAnimationComponent|GetAnimInstance (Variables|Default|GetAnimationComponent)) (Variables|Edit|Getdamaged) "None")
      (Rendering|SetVisibility (Variables|Default|GetWidget) true false)
      (Utilities|FlowControl|RetriggerableDelay 1.0)
      (Variables|Donotedit|Setenemydamaged false))))

(fn ConstructionScript)