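; NPC actor that shows lines from its Dialogue array in a Dialog widget.
; Each Talk call advances Talkindex, creates and caches the widget on first use, and sets its text, with a hard-coded wrap after index 2.
; The Trigger component re-adds the cached widget when the player character enters and removes it on exit.
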(event OnComponentBeginOverlap(Trigger)
  (params (OverlappedComponent :type Primitive%20Component%20Object%20Reference) (OtherActor :type Actor%20Object%20Reference) (OtherComp :type Primitive%20Component%20Object%20Reference) (OtherBodyIndex :type Integer) (bFromSweep :type Boolean) (SweepResult :type Hit%20Result%20Structure%20%28by%20ref%29))
  (if (== OtherActor (Game|GetPlayerCharacter 0))
    (Utilities|IsValid (Variables|Default|GetUI)
      (:Is%20Valid
        (UserInterface|Viewport|AddtoViewport (Variables|Default|GetUI) 0)))))

(event OnComponentEndOverlap(Trigger)
  (params (OverlappedComponent :type Primitive%20Component%20Object%20Reference) (OtherActor :type Actor%20Object%20Reference) (OtherComp :type Primitive%20Component%20Object%20Reference) (OtherBodyIndex :type Integer))
  (bind _ui (Variables|Default|GetUI))
  (if (== OtherActor (Game|GetPlayerCharacter 0))
    (Utilities|IsValid _ui
      (:Is%20Valid
        (Widget|RemovefromParent _ui)))))

(event EventTalk
  (Math|Integer|IncrementInt (Variables|Default|Gettalkindex)
    (:%20%20
      (if (<= (Variables|Default|Gettalkindex) (Utilities|Array|Length (Variables|Default|GetDialogue)))
        (Variables|Default|GetUI
          (:then
            _)
          (:else
            (bind _returnvalue (UserInterface|CreateWidget "/Game/Dialogue/Dialog.Dialog_C" (Game|GetPlayerController 0)))
            (bind _output_get (Variables|Default|SetUI _returnvalue))
            (UserInterface|Viewport|AddtoViewport _output_get 0)))
        (Rendering|Components|TextRender|SetText (Variables|/Game/Dialogue/Dialog.Dialog_C|GetTalkText (Variables|Default|GetUI)) (Utilities|Text|ToText(String) (Utilities|Array|Get(acopy) (Variables|Default|GetDialogue) (Variables|Default|Gettalkindex))))
        (if (== (Variables|Default|Gettalkindex) 2)
          (Variables|Default|Settalkindex -1))))))

(fn ConstructionScript)